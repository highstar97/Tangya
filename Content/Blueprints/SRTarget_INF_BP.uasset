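; Shooting target actor that awards 6 to 10 points for each SRBullet that overlaps it.
; On overlap, it compares the bullet's position with a scoring center offset below the actor origin, sends the score to SRPlayerController's EarnScore, then destroys the bullet.
; CheckScore grades hits on the Y-Z plane, using horizontal bands within a central vertical span and radial distance beyond it.
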(event Custom|OnActorHit_Event
  (params (SelfActor :type Actor%20Object%20Reference) (OtherActor :type Actor%20Object%20Reference) (NormalImpulse :type Vector) (Hit :type Hit%20Result%20Structure%20%28by%20ref%29)))

(event EventBeginPlay
  (|CallParentFunction) ; 지금 이 노드는 비활성 상태입니다. \n핀을 끌어서 다른 노드를 연결하면 활성화됩니다.
)

(event Collision|EventActorBeginOverlap
  (params (OtherActor :type Actor%20Object%20Reference))
  ;[1 1 1] 점수 확인
  (bind _assrbullet (Utilities|Casting|CastToSRBullet OtherActor))
  (bind _output_get (Variables|Bullet|SetBullet _assrbullet))
  (bind _score (CallFunction|CheckScore (- (Transformation|GetActorLocation self) "0, 0,118.000000") (Transformation|GetActorLocation _output_get)))
  (bind _assrplayer_controller (Utilities|Casting|CastToSRPlayerController (Game|GetPlayerController 0)))
  (Class|SRPlayerController|EarnScore _assrplayer_controller (Math|Conversions|ToFloat(Integer) _score))
  (Actor|DestroyActor (Variables|Bullet|GetBullet)))

(event EventTick
  (params (DeltaSeconds :type Float%20%28single-precision%29)))

(fn ConstructionScript
  (|CallParentFunction))

(fn CheckScore
  (params (TargetVector :type Vector) (BulletVector :type Vector))
  (bind _returnvalue (- TargetVector BulletVector))
  (bind (_x _y _z) (Math|Vector|BreakVector _returnvalue))
  (LocalVariables|SetabsY (Math|Float|Absolute(Float) _y))
  (LocalVariables|SetabsZ (Math|Float|Absolute(Float) _z))
  (if (<= (LocalVariables|GetabsZ) 17.5)
    ;[1 1 1] Can be divided by rectangle
    (if (<= (LocalVariables|GetabsY) 4.5)
      (LocalVariables|SetEarned%20Score 10)
      (elif (<= (LocalVariables|GetabsY) 11.0)
        (LocalVariables|SetEarned%20Score 9)
        (elif (<= (LocalVariables|GetabsY) 17.5)
          (LocalVariables|SetEarned%20Score 8)
          (elif (<= (LocalVariables|GetabsY) 24.0)
            (LocalVariables|SetEarned%20Score 7)
            (else
              (LocalVariables|SetEarned%20Score 6))))))
    (else
      ;[1 1 1] Divided by Circle
      (LocalVariables|SetabsDistance (Math|Vector|Distance(Vector) (+ TargetVector "0, 0,17.500000") (+ TargetVector (Math|Vector|MakeVector 0.0 (LocalVariables|GetabsY) (LocalVariables|GetabsZ)))))
      (if (<= (LocalVariables|GetabsDistance) 4.5)
        (LocalVariables|SetEarned%20Score 10)
        (elif (<= (LocalVariables|GetabsDistance) 11.0)
          (LocalVariables|SetEarned%20Score 9)
          (elif (<= (LocalVariables|GetabsDistance) 17.5)
            (LocalVariables|SetEarned%20Score 8)
            (elif (<= (LocalVariables|GetabsDistance) 24.0)
              (LocalVariables|SetEarned%20Score 7)
              (else
                (LocalVariables|SetEarned%20Score 6))))))))
  (return (LocalVariables|GetEarned%20Score)))