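; SRCharacterBlueprint is a character Blueprint that adds an aim-down-sight camera toggle.
; Each press of the AimDownSight input checks whether the main Camera is active, then swaps between it and ADSCamera by deactivating one and activating the other.
; Release is not handled, so aiming is a toggle rather than a hold.
; BeginPlay, overlap, Tick and the construction script are empty.
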(event EventBeginPlay)

(event Collision|EventActorBeginOverlap
  (params (OtherActor :type Actor%20Object%20Reference)))

(event EventTick
  (params (DeltaSeconds :type Float%20%28single-precision%29)))

(event Input|ActionEvents|InputActionAimDownSight
  (params (Key :type Key%20Structure :default "None"))
  (:Pressed
    (if (Components|Activation|IsActive (Variables|Default|GetCamera))
      (Components|Activation|Deactivate (Variables|Default|GetCamera))
      (Components|Activation|Activate (Variables|Default|GetADSCamera) false)
      (else
        (Components|Activation|Deactivate (Variables|Default|GetADSCamera))
        (Components|Activation|Activate (Variables|Default|GetCamera) false)))))

(fn ConstructionScript)